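; BP_ScannableObject is a world object the player scans to add its name, description and icon to a BP_Ship log.
; A trigger toggles the scan indicator when the first-person character enters or leaves.
; StartScan, called externally, shows a progress widget and runs function-name timers for completion, bar updates and distance checks.
; Moving out of range resets progress and removes the widget, but leaves the CompleteScan timer running.
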(event `self.ReceiveTick`
  (params (DeltaSeconds :type "Float (single-precision)")))

(event `self.ScanTrigger.OnComponentBeginOverlap`
  (params (OverlappedComponent :type "PrimitiveComponent Object Reference") (OtherActor :type "Actor Object Reference") (OtherComp :type "PrimitiveComponent Object Reference") (OtherBodyIndex :type Integer) (bFromSweep :type Boolean) (SweepResult :type "HitResult Structure (by ref)"))
  ;[1 1 1] Set Indicator Visible
  (cast `/Game/FirstPerson/Blueprints/BP_FirstPersonCharacter` OtherActor)
  (`SceneComponent.SetVisibility` (`self.ScanIndicator`) true false))

(event `self.ScanTrigger.OnComponentEndOverlap`
  (params (OverlappedComponent :type "PrimitiveComponent Object Reference") (OtherActor :type "Actor Object Reference") (OtherComp :type "PrimitiveComponent Object Reference") (OtherBodyIndex :type Integer))
  ;[0.675 0.6522 1] Set Indicator Invisible
  (cast `/Game/FirstPerson/Blueprints/BP_FirstPersonCharacter` OtherActor)
  (`SceneComponent.SetVisibility` (`self.ScanIndicator`) false false))

(event `StartScan`
  ;[1 0.9629 0.6069] Start Scan
  (set `self.ElapsedTime` 0.0)
  (set `self.Progress` 0.0)
  (set `self.isScanning` true)
  (bind _returnvalue (`|CreateWidget` "/Game/UI/WB_ScanProgress.WB_ScanProgress_C"))
  (`UserWidget.AddToViewport` _returnvalue 0)
  (set `self.ScanProgressWidget` _returnvalue)
  (`KismetSystemLibrary.K2_SetTimer` null "CompleteScan" (`self.ScanTime`))
  (`KismetSystemLibrary.K2_SetTimer` null "UpdateScanBarProgress" 0.1 true)
  (`KismetSystemLibrary.K2_SetTimer` null "CheckDistance" 0.05 true))

(event `UpdateScanBarProgress`
  ;[0.5224 0.151 1] Update Scan Bar Progress
  (bind _output_get (set `self.ElapsedTime` (+ (`self.ElapsedTime`) 0.1)))
  (bind _output_get_2 (set `self.Progress` (/ _output_get (`self.ScanTime`))))
  (`/Game/UI/WB_ScanProgress.UpdateScanner` (`self.ScanProgressWidget`) _output_get_2)
  (if (>= (`self.Progress`) 1.0)
    (`KismetSystemLibrary.K2_ClearTimer` null "UpdateScanBarProgress")))

(event `CompleteScan`
  ;[0.4199 1 0.4372] Complete Scan
  (set `self.isScanning` false)
  (set `self.IsScanned` true)
  (`Widget.RemoveFromParent` (`self.ScanProgressWidget`))
  (bind _returnvalue (`GameplayStatics.GetActorOfClass` "/Game/FirstPerson/Blueprints/BP_Ship.BP_Ship_C"))
  (bind _asbp_ship (cast `/Game/FirstPerson/Blueprints/BP_Ship` _returnvalue)
    (:`then`
      (`/Game/FirstPerson/Blueprints/BP_Ship.AddScanEntry` _asbp_ship (`self.ObjectName`) (`self.ObjectDescription`) (`self.ObjectIcon`)))
    (:`CastFailed`
      (`KismetSystemLibrary.PrintString` "failes"))))

(event `CheckDistance`
  ;[1 0.1187 0.7187] Check Distance For Scan
  (if (>= (`KismetMathLibrary.VSize` (- (`self.K2_GetActorLocation` (`GameplayStatics.GetPlayerCharacter` 0)) (`self.K2_GetActorLocation`))) 300.0)
    (`self.ScanInterrupted`)))

(event `ScanInterrupted`
  ;[1 0.03209 0] Interrupting Scan
  (set `self.isScanning` false)
  (`KismetSystemLibrary.K2_ClearTimer` null "UpdateScanBarProgress")
  (`KismetSystemLibrary.K2_ClearTimer` null "CheckDistance")
  (set `self.Progress` 0.0)
  (set `self.ElapsedTime` 0.0)
  (`Widget.RemoveFromParent` (`self.ScanProgressWidget`)))

(fn `UserConstructionScript`)