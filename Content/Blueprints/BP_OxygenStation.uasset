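; BP_OxygenStation is a refill station where the first-person character regains oxygen.
; Entering its Box sets IsAtRefillStation and starts a looping timer on the character's RefillOxygen function; leaving clears both.
; On BeginPlay it finds a BP_OxygenStationIndicator in the level by class.
; Each Tick it re-rotates that indicator with a look-at whose target is the indicator-minus-player offset vector, rather than the player's position.
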(event `self.ReceiveBeginPlay`
  (bind _returnvalue (`GameplayStatics.GetActorOfClass` "/Game/Blueprints/BP_OxygenStationIndicator.BP_OxygenStationIndicator_C"))
  (set `self.OxygenStationIndicator` _returnvalue))

(event `self.ReceiveTick`
  (params (DeltaSeconds :type "Float (single-precision)"))
  (bind _oxygenstationindicator (`self.OxygenStationIndicator`))
  (bind _returnvalue (`self.K2_GetActorLocation` (`self.OxygenStationIndicator`)))
  (`self.K2_SetActorRotation` _oxygenstationindicator (`KismetMathLibrary.FindLookAtRotation` _returnvalue (- _returnvalue (`self.K2_GetActorLocation` (`GameplayStatics.GetPlayerPawn` 0)))) false)
  (set `self.OxygenStationIndicator` _oxygenstationindicator))

(event `self.Box.OnComponentBeginOverlap`
  (params (OverlappedComponent :type "PrimitiveComponent Object Reference") (OtherActor :type "Actor Object Reference") (OtherComp :type "PrimitiveComponent Object Reference") (OtherBodyIndex :type Integer) (bFromSweep :type Boolean) (SweepResult :type "HitResult Structure (by ref)"))
  (bind _asbp_first_person_character (cast `/Game/FirstPerson/Blueprints/BP_FirstPersonCharacter` OtherActor))
  (`|ExecutionSequence`
    (:`then_0`
      (`KismetSystemLibrary.K2_SetTimer` _asbp_first_person_character "RefillOxygen" 0.5 true))
    (:`then_1`
      (set `/Game/FirstPerson/Blueprints/BP_FirstPersonCharacter.isAtRefillStation` true _asbp_first_person_character))))

(event `self.Box.OnComponentEndOverlap`
  (params (OverlappedComponent :type "PrimitiveComponent Object Reference") (OtherActor :type "Actor Object Reference") (OtherComp :type "PrimitiveComponent Object Reference") (OtherBodyIndex :type Integer))
  (bind _asbp_first_person_character (cast `/Game/FirstPerson/Blueprints/BP_FirstPersonCharacter` OtherActor))
  (`|ExecutionSequence`
    (:`then_0`
      (`KismetSystemLibrary.K2_ClearTimer` _asbp_first_person_character "RefillOxygen"))
    (:`then_1`
      (set `/Game/FirstPerson/Blueprints/BP_FirstPersonCharacter.isAtRefillStation` false _asbp_first_person_character))))

(fn `UserConstructionScript`)