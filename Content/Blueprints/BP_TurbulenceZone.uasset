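; Turbulence zone actor that buffets any BP_Ship inside its TurbulenceArea with randomized forces.
; On overlap it flags the ship and starts two looping timers: the ship's UpdateResistanceEnergy and its own ApplyTurbulenceForce.
; Each force tick applies mass-independent acceleration to overlapping ships' models, combining a base TurbulenceForce with random jitter scaled by ForceRandomness.
; Leaving clears the ship's flag, but neither timer is stopped here.
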(event `self.TurbulenceArea.OnComponentBeginOverlap`
  (params (OverlappedComponent :type "PrimitiveComponent Object Reference") (OtherActor :type "Actor Object Reference") (OtherComp :type "PrimitiveComponent Object Reference") (OtherBodyIndex :type Integer) (bFromSweep :type Boolean) (SweepResult :type "HitResult Structure (by ref)"))
  (bind _asbp_ship (cast `/Game/FirstPerson/Blueprints/BP_Ship` OtherActor))
  (set `/Game/FirstPerson/Blueprints/BP_Ship.IsInTurbulenceZone` true _asbp_ship)
  (`KismetSystemLibrary.K2_SetTimer` _asbp_ship "UpdateResistanceEnergy" 0.1 true)
  (`KismetSystemLibrary.K2_SetTimer` null "ApplyTurbulenceForce" (`self.ForceFrequency`) true))

(event `ApplyTurbulenceForce`
  (for _array_element (`self.GetOverlappingActors` "/Game/FirstPerson/Blueprints/BP_Ship.BP_Ship_C")
    (bind _asbp_ship (cast `/Game/FirstPerson/Blueprints/BP_Ship` _array_element))
    (`KismetSystemLibrary.PrintString` "cast")
    (`PrimitiveComponent.AddForce` (`/Game/FirstPerson/Blueprints/BP_Ship.Ship Model` _asbp_ship) (+ (`self.TurbulenceForce`) (* (`KismetMathLibrary.MakeVector` (`KismetMathLibrary.RandomFloatInRange` -1.0 1.0) (`KismetMathLibrary.RandomFloatInRange` -1.0 1.0) (`KismetMathLibrary.RandomFloatInRange` -1.0 1.0)) (`self.ForceRandomness`))) "None" true)))

(event `self.TurbulenceArea.OnComponentEndOverlap`
  (params (OverlappedComponent :type "PrimitiveComponent Object Reference") (OtherActor :type "Actor Object Reference") (OtherComp :type "PrimitiveComponent Object Reference") (OtherBodyIndex :type Integer))
  (bind _asbp_ship (cast `/Game/FirstPerson/Blueprints/BP_Ship` OtherActor))
  (set `/Game/FirstPerson/Blueprints/BP_Ship.IsInTurbulenceZone` false _asbp_ship))

(event `self.ReceiveBeginPlay`)

(fn `UserConstructionScript`)